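; Auto-targeting turret that tracks and damages the nearest "Ennemie"-tagged actor, with logic driven by the server.
; A detection sphere maintains the candidate list, from which a looping timer picks the closest target.
; Tick smoothly yaws the gun toward it or back to default, drawing debug arrows to candidates.
; A fire timer line-traces from the muzzle, ignoring other turrets, and directly subtracts BP_Ennemi health.
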(event `self.ReceiveTick`
  (params (DeltaSeconds :type "Float (single-precision)"))
  (bind _bestactor (`self.BestActor`))
  (bind (_returnvalue_x _returnvalue_y _returnvalue_z) (`KismetMathLibrary.BreakVector` (`SceneComponent.K2_GetComponentLocation` (`self.muzzle`))))
  (`/Engine/EditorBlueprintResources/ActorMacros.Switch Has Authority`
    (:`Authority`
      (set `self.Delta Seconds` DeltaSeconds)
      (if (`self.Has A Target ?`)
        (`/Engine/EditorBlueprintResources/StandardMacros.IsValid` _bestactor
          (:`Is Valid`
            (bind _output_get (set `self.CurrentRotation` (`KismetMathLibrary.RInterpTo` (`self.CurrentRotation`) (`KismetMathLibrary.FindLookAtRotation` (`self.K2_GetActorLocation`) (`self.K2_GetActorLocation` _bestactor)) (`self.Delta Seconds`) (`self.Interp Speed`))))
            (`SceneComponent.K2_SetWorldRotation` (`self.Gun_Turret`) (`KismetMathLibrary.MakeRotator` 0.0 0.0 (.yaw _output_get)) false false)
            ; Blue arrows
            (for _array_element (`self.Candidats`)
              (`/Engine/EditorBlueprintResources/StandardMacros.IsValid` _array_element
                (:`Is Valid`
                  (bind (_returnvalue_x_2 _returnvalue_y_2) (`KismetMathLibrary.BreakVector` (`self.K2_GetActorLocation` _array_element)))
                  (`KismetSystemLibrary.DrawDebugArrow` (`KismetMathLibrary.MakeVector` _returnvalue_x _returnvalue_y _returnvalue_z) (`KismetMathLibrary.MakeVector` _returnvalue_x_2 _returnvalue_y_2 _returnvalue_z) 30.0 (struct :`G` 0.992904 :`B` 1.0 :`A` 1.0) 0.0 2.0))))))
        (else
          ; NO ACTOR == GO BACK TO DEFAULT ROTATION
          (bind _output_get_2 (set `self.CurrentRotation` (`KismetMathLibrary.RInterpTo` (`self.CurrentRotation`) (`self.DefaultRotation`) (`self.Delta Seconds`) (`self.Interp Speed`))))
          (`SceneComponent.K2_SetRelativeRotation` (`self.Gun_Turret`) (`KismetMathLibrary.MakeRotator` 0.0 0.0 (.yaw _output_get_2)) false false))))))

(event `self.DetectionSphere.OnComponentBeginOverlap`
  (params (OverlappedComponent :type "PrimitiveComponent Object Reference") (OtherActor :type "Actor Object Reference") (OtherComp :type "PrimitiveComponent Object Reference") (OtherBodyIndex :type Integer) (bFromSweep :type Boolean) (SweepResult :type "HitResult Structure (by ref)"))
  ; TARGET ENNEMI IN PHERE = PUT IN LIST, IS NOT IN ENYMORE = REMOVE
  ;;[0.3594 0.3594 0.3594] begin overlap
  (`/Engine/EditorBlueprintResources/ActorMacros.Switch Has Authority`
    (:`Authority`
      (if (`self.ActorHasTag` OtherActor "Ennemie")
        (`KismetArrayLibrary.Array_Add` (`self.Candidats`) OtherActor)))))

(event `self.DetectionSphere.OnComponentEndOverlap`
  (params (OverlappedComponent :type "PrimitiveComponent Object Reference") (OtherActor :type "Actor Object Reference") (OtherComp :type "PrimitiveComponent Object Reference") (OtherBodyIndex :type Integer))
  ; TARGET ENNEMI IN PHERE = PUT IN LIST, IS NOT IN ENYMORE = REMOVE
  ;;[0.3594 0.3594 0.3594] End Overlap
  (`/Engine/EditorBlueprintResources/ActorMacros.Switch Has Authority`
    (:`Authority`
      (if (`self.ActorHasTag` OtherActor "Ennemie")
        (`KismetArrayLibrary.Array_RemoveItem` (`self.Candidats`) OtherActor)))))

(event `SHOOT`
  (bind _returnvalue (`SceneComponent.K2_GetComponentLocation` (`self.muzzle`)))
  ; FIRE IF HAS TARGET
  (if (`self.Has A Target ?`)
    (bind _outactors (`GameplayStatics.GetAllActorsOfClass` "BP_Turret_C"))
    ;;[0.3594 0.3594 0.3594] line trace
    (bind _outhit (`KismetSystemLibrary.LineTraceSingle` _returnvalue (+ _returnvalue (* (`SceneComponent.GetForwardVector` (`self.muzzle`)) (`self.ShootRange`))) "TraceTypeQuery1" false _outactors (`self.Draw Debug Type`)))
    ;;[0.3594 0.3594 0.3594] is a ennemi ?
    (`/Engine/EditorBlueprintResources/StandardMacros.IsValid` (`.HitActor` (`GameplayStatics.BreakHitResult` _outhit))
      (:`Is Valid`
        (if (`self.ActorHasTag` (`.HitActor` (`GameplayStatics.BreakHitResult` _outhit)) "Ennemie")
          ;;[0.3594 0.3594 0.3594] remove HP
          (bind _asbp_ennemi (cast `/Game/Blueprints/BP_Ennemi` (`.HitActor` (`GameplayStatics.BreakHitResult` _outhit))))
          (set `/Game/Blueprints/BP_Ennemi.CurentHealth` (- (`/Game/Blueprints/BP_Ennemi.CurentHealth` _asbp_ennemi) (`self.degats`)) _asbp_ennemi))))))

(event `self.ReceiveBeginPlay`
  ; begin play
  (if (`self.HasAuthority`)
    ;;[0.3594 0.3594 0.3594] disable collision for dun
    (`PrimitiveComponent.SetCollisionEnabled` (`self.Gun_Turret`) "NoCollision")
    ;;[0.3594 0.3594 0.3594] set the size of the detection radius
    (`SphereComponent.SetSphereRadius` (`self.DetectionSphere`) (`self.DetectionRadius`) true)
    ;;[0.3594 0.3594 0.3594] set current target to none
    (set `self.CurrentTarget` null)
    (`KismetSystemLibrary.K2_SetTimerDelegate` (delegate `Best Target Refresh`) (`self.RefreshRate`) true)
    (`KismetSystemLibrary.K2_SetTimerDelegate` (delegate `SHOOT`) (`self.FireRate`) true)))

(event `Best Target Refresh`
  (bind _bestactor (`self.BestActor`))
  ; get closer target
  (`/Engine/EditorBlueprintResources/ActorMacros.Switch Has Authority`
    (:`Authority`
      (if (== (`KismetArrayLibrary.Array_Length` (`self.Candidats`)) 0)
        (set `self.Has A Target ?` false)
        (else
          (set `self.BestActor` null)
          (set `self.BestDistance` 10000.0)
          (for _array_element (`self.Candidats`)
            (`/Engine/EditorBlueprintResources/StandardMacros.IsValid` _array_element
              (:`Is Valid`
                (bind _returnvalue (`KismetMathLibrary.Vector_Distance` (`self.K2_GetActorLocation`) (`self.K2_GetActorLocation` _array_element)))
                (if (< _returnvalue (`self.BestDistance`))
                  (set `self.BestActor` _array_element)
                  (set `self.BestDistance` _returnvalue)))))
          (`/Engine/EditorBlueprintResources/StandardMacros.IsValid` _bestactor
            (:`Is Valid`
              (set `self.CurrentTarget` _bestactor)
              (set `self.Has A Target ?` true))
            (:`Is Not Valid`
              (set `self.CurrentTarget` null))))))))

(fn `OnRep_CurrentRotation`)

(fn `UserConstructionScript`)