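; BP_GameModeGAME is a Game Mode that opens the main menu and tracks joining players.
; On BeginPlay it has the persistent BP_GameInstance show the menu, since the mode does not survive level changes, and enables cursor and click events.
; PostLogin, marked unfinished and broken, prints the player count and casts the pawn to BP_Character.
; The per-player body material assignment is disconnected and never runs.
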(event `self.ReceiveBeginPlay`
  (bind _returnvalue (`GameplayStatics.GetPlayerController` 0))
  ; GAMEMODE est pas persistant entre level, donc il demande a game instance de faire apparaitre le menu principal, car game instance est persistant, et vas dire si oui ou non il peut afficher le menu.
  (bind _asbp_game_instance (cast `/Game/Blueprints/BP_GameInstance` (`GameplayStatics.GetGameInstance`)))
  (`/Game/Blueprints/BP_GameInstance.MakeMainMenuAppear` _asbp_game_instance)
  (set `PlayerController.bShowMouseCursor` true _returnvalue)
  (set `PlayerController.bEnableClickEvents` true _returnvalue))

(event `self.K2_PostLogin`
  (params (NewPlayer :type "PlayerController Object Reference"))
  ;[1 0 0 0.5] WORK IN PROGRESS JULES - DOES NOT WORK
  (`KismetSystemLibrary.PrintString` "hello new player")
  (`KismetSystemLibrary.PrintString` (`KismetStringLibrary.Conv_IntToString` (`KismetArrayLibrary.Array_Length` (`GameStateBase.PlayerArray` (`GameplayStatics.GetGameState`)))) true true (struct :`G` 0.66 :`B` 1.0 :`A` 1.0) 20.0)
  (bind _asbp_character (cast `/Game/Blueprints/BP_Character` (`Controller.K2_GetPawn` NewPlayer))))

(fn `UserConstructionScript`)