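; BP_Ennemi is an AI enemy that keeps moving toward randomly chosen BPP_Turret actors until its health runs out.
; BeginPlay initialises its health bar widget and starts the AI MoveTo loop, which picks another random turret after each success or failure.
; Tick turns the health bar toward the BP_Character camera and broadcasts current health through a dispatcher.
; At zero health, a one-time timeline animates the actor's scale, then destroys it.
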(event `BeanDisapear`
  (bind (_direction _newtrack_0) (`Timeline|Timeline` :!via `PlayFromStart`)
    (:`Update`
      (`self.SetActorScale3D` (`KismetMathLibrary.MakeVector` _newtrack_0 _newtrack_0 _newtrack_0)))
    (:`Finished`
      (`self.K2_DestroyActor`))))

(event `self.ReceiveTick`
  (params (DeltaSeconds :type "Float (single-precision)"))
  (bind _healthbar (`self.HealthBar`))
  (bind _returnvalue (`GameplayStatics.GetActorOfClass` "/Game/Blueprints/BP_Character/BP_Character.BP_Character_C"))
  (`/Engine/EditorBlueprintResources/StandardMacros.IsValid` _returnvalue
    (:`Is Valid`
      (`SceneComponent.K2_SetWorldRotation` _healthbar (`KismetMathLibrary.FindLookAtRotation` (`SceneComponent.K2_GetComponentLocation` _healthbar) (`SceneComponent.K2_GetComponentLocation` (`/Game/Blueprints/BP_Character/BP_Character.Camera` _returnvalue))) false false))
    (:`Is Not Valid`
      _))
  (`self.ED_HealthUpdate` (`self.CurentHealth`) (`self.MaxHealth`))
  (if (<= (`self.CurentHealth`) 0.0)
    (`/Engine/EditorBlueprintResources/StandardMacros.DoOnce` false
      (:`Completed`
        (`self.BeanDisapear`)))))

(event `GET A RANDOM POINT`
  (bind _outactors (`GameplayStatics.GetAllActorsOfClass` "/Game/Blueprints/BP_Props/BPP_Turret.BPP_Turret_C" :!label _label))
  (bind _outitem (`KismetArrayLibrary.Array_Random` _outactors))
  (`/Engine/EditorBlueprintResources/StandardMacros.IsValid` _outitem
    (:`Is Valid`
      (`|AIMoveTo` self (`self.K2_GetActorLocation` _outitem) _outitem
        (:`OnSuccess`
          _)
        (:`OnFail`
          _))
      (`self.GET A RANDOM POINT`))))

(event `self.ReceiveBeginPlay`
  (bind _ashealth_bar (cast `/Game/Blueprints/Widgets/Widget_Ennemi/HealthBar` (`WidgetComponent.GetWidget` (`self.HealthBar`))))
  (`/Game/Blueprints/Widgets/Widget_Ennemi/HealthBar.Initialise` _ashealth_bar self)
  (goto _label))

(fn `UserConstructionScript`)