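; Automatic turret prop that, when activated, targets and shoots actors tagged "Ennemie" within its detection sphere.
; Overlap events (authority only) and a looping rescan timer fill the enemy list, from which the closest becomes the target.
; Tick smoothly yaws the gun toward the target, or back to default when none.
; A fire-rate timer sphere-traces for a clear shot, then line-traces to subtract BP_Ennemi health directly, with debug drawing.
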(event `self.ReceiveBeginPlay`
  ; begin play
  (if (`self.ACTIVATE_TURRET?`)
    ;;[0.3594 0.3594 0.3594] disable collision for dun
    (`PrimitiveComponent.SetCollisionEnabled` (`self.Gun_Turret`) "NoCollision")
    ;;[0.3594 0.3594 0.3594] set the size of the detection radius
    (`SphereComponent.SetSphereRadius` (`self.DetectionSphere`) (`self.Dectection_Radius`) true)
    ;;[0.3613 0.3613 0.3613] refresh la target
    (`KismetSystemLibrary.K2_SetTimer` null "Get_The_Closest_Target" (`self.Ennemy_Refresh_Rate`) true)
    ;;[0.3613 0.3613 0.3613] regarde si peut tirer et tire quand target est visible
    (`KismetSystemLibrary.K2_SetTimer` null "PreShoot/Shoot" (`self.Turret_Fire_Rate`) true)))

(event `self.DetectionSphere.OnComponentBeginOverlap`
  (params (OverlappedComponent :type "PrimitiveComponent Object Reference") (OtherActor :type "Actor Object Reference") (OtherComp :type "PrimitiveComponent Object Reference") (OtherBodyIndex :type Integer) (bFromSweep :type Boolean) (SweepResult :type "HitResult Structure (by ref)"))
  ;[0.15 0.15 0.15 0.5 50] TARGET ENNEMI IN PHERE = PUT IN LIST, IS NOT IN ENYMORE = REMOVE
  ;;[0.3594 0.3594 0.3594] begin overlap
  (`/Engine/EditorBlueprintResources/ActorMacros.Switch Has Authority`
    (:`Authority`
      (if (`self.ActorHasTag` OtherActor "Ennemie")
        (`KismetArrayLibrary.Array_Add` (`self.Ennemy_In_Range`) OtherActor)))))

(event `self.DetectionSphere.OnComponentEndOverlap`
  (params (OverlappedComponent :type "PrimitiveComponent Object Reference") (OtherActor :type "Actor Object Reference") (OtherComp :type "PrimitiveComponent Object Reference") (OtherBodyIndex :type Integer))
  ;[0.15 0.15 0.15 0.5 50] TARGET ENNEMI IN PHERE = PUT IN LIST, IS NOT IN ENYMORE = REMOVE
  ;;[0.3594 0.3594 0.3594] End Overlap
  (`/Engine/EditorBlueprintResources/ActorMacros.Switch Has Authority`
    (:`Authority`
      (if (`self.ActorHasTag` OtherActor "Ennemie")
        (`KismetArrayLibrary.Array_RemoveItem` (`self.Ennemy_In_Range`) OtherActor)))))

(event `Aim to Ennemi`
  (bind _current_target (`self.Current_Target`))
  ;[0.15 0.15 0.15 0.5 40] AIM TO ENNEMI
  (`/Engine/EditorBlueprintResources/StandardMacros.IsValid` _current_target
    (:`Is Valid`
      (bind _output_get (set `self.Current_Turret_Rotation` (`KismetMathLibrary.RInterpTo` (`self.Current_Turret_Rotation`) (`KismetMathLibrary.FindLookAtRotation` (`self.K2_GetActorLocation`) (`self.K2_GetActorLocation` _current_target)) (`self.Delta_Seconds`) (`self.Turret_Rotation_Speed`))))
      (`SceneComponent.K2_SetWorldRotation` (`self.Gun_Turret`) (`KismetMathLibrary.MakeRotator` 0.0 0.0 (.yaw _output_get)) false false))))

(event `self.ReceiveTick`
  (params (DeltaSeconds :type "Float (single-precision)"))
  ; EVENT TICK
  (if (`self.ACTIVATE_TURRET?`)
    (set `self.Delta_Seconds` DeltaSeconds)
    (if (`self.Has_A_Target ?`)
      (`self.Aim to Ennemi`)
      (else
        (`self.Go Default ROT`)))))

(event `Go Default ROT`
  ;[0.15 0.15 0.15 0.5 40] NO ACTOR == GO BACK TO DEFAULT ROTATION
  (bind _output_get (set `self.Current_Turret_Rotation` (`KismetMathLibrary.RInterpTo` (`self.Current_Turret_Rotation`) (`self.Default_Turret_Rotation`) (`self.Delta_Seconds`) (`self.Turret_Rotation_Speed`))))
  (`SceneComponent.K2_SetRelativeRotation` (`self.Gun_Turret`) (`KismetMathLibrary.MakeRotator` 0.0 0.0 (.yaw _output_get)) false false))

(fn `Get_The_Closest_Target`
  (locals (Closest_Target :type "Actor Object Reference") (Best_Distance :type "Float (double-precision)" :default 5000.0))
  (bind _closest_target (`local.Closest_Target`))
  ; GET THE MISSING ENNEMY AND SET THE CLOSEST ONE THE CURRENT ONE
  ;; look for any missing actors
  (bind _outactors (`GameplayStatics.GetAllActorsOfClassWithTag` "/Script/Engine.Actor" "Ennemie"))
  (for _array_element _outactors
    (`/Engine/EditorBlueprintResources/StandardMacros.IsValid` _array_element
      (:`Is Valid`
        (if (`PrimitiveComponent.IsOverlappingActor` (`self.DetectionSphere`) _array_element)
          (`KismetArrayLibrary.Array_Add` (`self.Ennemy_In_Range`) _array_element)))))
  ;; 0 ennemy == no target
  (if (== (`KismetArrayLibrary.Array_Length` (`self.Ennemy_In_Range`)) 0)
    (set `self.Has_A_Target ?` false)
    (else
      (set `local.Closest_Target` null)
      (set `local.Best_Distance` 5000.0)
      ;; get the closest ennemy out of all actors
      (for _array_element_2 (`self.Ennemy_In_Range`)
        (`/Engine/EditorBlueprintResources/StandardMacros.IsValid` _array_element_2
          (:`Is Valid`
            (bind _returnvalue (`KismetMathLibrary.Vector_Distance` (`self.K2_GetActorLocation`) (`self.K2_GetActorLocation` _array_element_2)))
            (if (< _returnvalue (`local.Best_Distance`))
              (set `local.Closest_Target` _array_element_2)
              (set `local.Best_Distance` _returnvalue)))))
      ;; set closest ennemy the current one
      (`/Engine/EditorBlueprintResources/StandardMacros.IsValid` _closest_target
        (:`Is Valid`
          (set `self.Current_Target` _closest_target)
          (set `self.Has_A_Target ?` true))
        (:`Is Not Valid`
          (set `self.Current_Target` null))))))

(fn `PreShoot/Shoot`
  (bind _returnvalue (`SceneComponent.K2_GetComponentLocation` (`self.muzzle`)))
  (bind _returnvalue_2 (`SceneComponent.K2_GetComponentLocation` (`self.muzzle`)))
  ;[0.3613 0.3613 0.3613] si il a une target.
  (if (`self.Has_A_Target ?`)
    ;[0.3613 0.3613 0.3613] Tir une sphere qui fait la taille de la bullet, si sa touche quoi que se soit qui n'est pas l'ennemi, il ne tireras pas.
    (bind _outhit (`KismetSystemLibrary.SphereTraceSingle` :`Start` _returnvalue_2 :`End` (+ _returnvalue_2 (* (`SceneComponent.GetForwardVector` (`self.muzzle`)) (`self.Bullet_Fly_Distance`))) :`Radius` (`self.Bullet_Radius`) :`TraceChannel` "TraceTypeQuery1" :`DrawDebugType` "ForDuration" :`TraceColor` (struct :`A` 1.0) :`TraceHitColor` (struct :`R` 0.584589 :`G` 0.982327 :`B` 1.0 :`A` 1.0) :`DrawTime` 0.1))
    (`/Engine/EditorBlueprintResources/StandardMacros.IsValid` (`.HitActor` (`GameplayStatics.BreakHitResult` _outhit))
      (:`Is Valid`
        (if (`self.ActorHasTag` (`.HitActor` (`GameplayStatics.BreakHitResult` _outhit)) "Ennemie")
          ;[0.3594 0.3594 0.3594] LINE TRACE DE LA BULLET
          (bind _outhit_2 (`KismetSystemLibrary.LineTraceSingle` :`Start` _returnvalue :`End` (+ _returnvalue (* (`SceneComponent.GetForwardVector` (`self.muzzle`)) (`self.Bullet_Fly_Distance`))) :`TraceChannel` "TraceTypeQuery1" :`DrawDebugType` "ForDuration" :`DrawTime` 0.5))
          ;[0.3594 0.3594 0.3594] DID BULLET TOUCH AN ENNEMY
          (`/Engine/EditorBlueprintResources/StandardMacros.IsValid` (`.HitActor` (`GameplayStatics.BreakHitResult` _outhit_2))
            (:`Is Valid`
              (if (`self.ActorHasTag` (`.HitActor` (`GameplayStatics.BreakHitResult` _outhit_2)) "Ennemie")
                ;[0.3594 0.3594 0.3594] IF YES, REMOVE HP TO TOUCHED ENNEMY
                (bind _asbp_ennemi (cast `/Game/Blueprints/BP_Ennemy/BP_Ennemi` (`.HitActor` (`GameplayStatics.BreakHitResult` _outhit_2))))
                (set `/Game/Blueprints/BP_Ennemy/BP_Ennemi.CurentHealth` (- (`/Game/Blueprints/BP_Ennemy/BP_Ennemi.CurentHealth` _asbp_ennemi) (`self.Bullet_Damage`)) _asbp_ennemi)))))))))

(fn `UserConstructionScript`)