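; BP_Weapon_Parent is a weapon Blueprint, named as a parent class, that fires hitscan shots at enemies.
; Its shoot event waits for Firerate, then line-traces on Visibility from the Muzzle along its forward vector, with random ShootError spread on the end point.
; A hit actor tagged "Ennemie" is cast to BP_Ennemi and has Degats subtracted directly from CurentHealth.
; The trace is debug-drawn for one frame.
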(event `shoot`
  (bind _muzzle (`self.Muzzle`))
  (bind _shooterror (`self.ShootError`))
  (bind _returnvalue (`SceneComponent.K2_GetComponentLocation` _muzzle))
  (bind _returnvalue_2 (* _shooterror -1.0))
  (`KismetSystemLibrary.Delay` (`self.firerate`))
  (bind _outhit (`KismetSystemLibrary.LineTraceSingle` :`Start` _returnvalue :`End` (+ _returnvalue (* (`SceneComponent.GetForwardVector` _muzzle) (`self.Shoot Distance`)) (`KismetMathLibrary.MakeVector` (`KismetMathLibrary.RandomFloatInRange` _returnvalue_2 _shooterror) (`KismetMathLibrary.RandomFloatInRange` _returnvalue_2 _shooterror) (`KismetMathLibrary.RandomFloatInRange` _returnvalue_2 _shooterror))) :`TraceChannel` "TraceTypeQuery1" :`DrawDebugType` "ForOneFrame"))
  (`/Engine/EditorBlueprintResources/StandardMacros.IsValid` (`.HitActor` (`GameplayStatics.BreakHitResult` _outhit))
    (:`Is Valid`
      (if (`self.ActorHasTag` (`.HitActor` (`GameplayStatics.BreakHitResult` _outhit)) "Ennemie")
        ;[0.3594 0.3594 0.3594] remove HP
        (bind _asbp_ennemi (cast `/Game/Blueprints/BP_Ennemy/BP_Ennemi` (`.HitActor` (`GameplayStatics.BreakHitResult` _outhit))))
        (set `/Game/Blueprints/BP_Ennemy/BP_Ennemi.CurentHealth` (- (`/Game/Blueprints/BP_Ennemy/BP_Ennemi.CurentHealth` _asbp_ennemi) (`self.degats`)) _asbp_ennemi)))))

(fn `UserConstructionScript`)