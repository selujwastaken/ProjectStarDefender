(event `self.ReceiveBeginPlay`
  (bind _asbp_character (cast `/Game/Blueprints/BP_Character/BP_Character` (`self.GetOwner`)))
  (bind _output_get (set `self.As BP Character` _asbp_character))
  (set `self.BP_Character_Camera` (`/Game/Blueprints/BP_Character/BP_Character.Camera` _output_get)))

(event `PreviewLoop`
  (bind _outactors (`GameplayStatics.GetAllActorsOfClass` "/Game/Blueprints/BP_Character/BP_Character.BP_Character_C"))
  (bind (_outhit _returnvalue) (`KismetSystemLibrary.LineTraceSingle` (`SceneComponent.K2_GetComponentLocation` (`self.BP_Character_Camera`)) (`/Game/Blueprints/BP_Character/BP_Character.MouseImpactPoint` (stale `self.ReceiveBeginPlay` _asbp_character)) "TraceTypeQuery1" false _outactors "None" true (struct :`R` 0.98045 :`B` 1.0 :`A` 1.0) (struct :`G` 1.0 :`A` 1.0) 0.05))
  (if _returnvalue
    (`|ExecutionSequence`
      (:`then_0`
        (`/Engine/EditorBlueprintResources/StandardMacros.DoOnce` false :!label _label
          (:`Completed`
            (bind _returnvalue_2 (`|AddComponentByClass` (`self.As BP Character`) "/Script/Engine.StaticMeshComponent" false (`self.Build_Preview_Transform`)))
            (bind _output_get (set `self.Preview_Mesh` _returnvalue_2))
            (`StaticMeshComponent.SetStaticMesh` _output_get (`self.MeshToDisplay`))
            (`PrimitiveComponent.SetCollisionEnabled` _output_get "NoCollision")
            (`PrimitiveComponent.SetMaterial` _output_get 0 "/Game/Materiaux/M_PreviewMesh_Correct.M_PreviewMesh_Correct"))))
      (:`then_1`
        (bind _output_get_2 (set `self.Build_Preview_Transform` (`KismetMathLibrary.MakeTransform` (`.Location` (`GameplayStatics.BreakHitResult` _outhit)) (`self.Target_Rot`))))
        (`SceneComponent.K2_SetWorldTransform` (`self.Preview_Mesh`) _output_get_2 false false)))))

(event `ResetBuildPreview`
  (goto _label :!via `Reset`))

(event `self.ReceiveTick`
  (params (DeltaSeconds :type "Float (single-precision)"))
  (`self.b_Build_Mode`
    (:`then`
      (`self.PreviewLoop`))
    (:`else`)))

(event `EnhancedInput|/Game/Blueprints/inputs/Input_Actions/Build_System/IA_Build_Rotate`
  (params (ActionValue :type "Float (double-precision)") (ElapsedSeconds :type "Float (double-precision)") (TriggeredSeconds :type "Float (double-precision)") (InputAction :type "InputAction Object Reference" :default "/Game/Blueprints/inputs/Input_Actions/Build_System/IA_Build_Rotate.IA_Build_Rotate"))
  (bind (_returnvalue_roll _returnvalue_pitch _returnvalue_yaw) (`KismetMathLibrary.BreakRotator` (`SceneComponent.K2_GetComponentRotation` (`self.Preview_Mesh`))))
  (bind (_returnvalue_roll_2 _returnvalue_pitch_2 _returnvalue_yaw_2) (`KismetMathLibrary.BreakRotator` (`SceneComponent.K2_GetComponentRotation` (`self.Preview_Mesh`))))
  (:`Triggered`
    (if (> ActionValue 0.0)
      (set `self.Target_Rot` (`KismetMathLibrary.MakeRotator` _returnvalue_roll_2 _returnvalue_pitch_2 (+ _returnvalue_yaw_2 1.0)))
      (else
        (set `self.Target_Rot` (`KismetMathLibrary.MakeRotator` _returnvalue_roll _returnvalue_pitch (- _returnvalue_yaw 1.0)))))))

(event `EnhancedInput|/Game/Blueprints/inputs/Input_Actions/Build_System/IA_Build_Toggle`
  (params (ActionValue :type "Float (double-precision)") (ElapsedSeconds :type "Float (double-precision)") (TriggeredSeconds :type "Float (double-precision)") (InputAction :type "InputAction Object Reference" :default "/Game/Blueprints/inputs/Input_Actions/Build_System/IA_Build_Toggle.IA_Build_Toggle"))
  (bind _as_bp_character (`self.As BP Character`))
  (bind _as_bp_character_2 (`self.As BP Character`))
  (:`Completed`
    (`/Engine/EditorBlueprintResources/StandardMacros.FlipFlop`
      (:`A`
        (set `self.b_Build_Mode` true)
        (`self.ResetBuildPreview`)
        (set `/Game/Blueprints/BP_Character/BP_Character.Can_Shoot` false _as_bp_character)
        (set `/Game/Blueprints/BP_Character/BP_Character.Can_PickUp_Item` false _as_bp_character))
      (:`B`
        (set `self.b_Build_Mode` false)
        (`StaticMeshComponent.SetStaticMesh` (`self.Preview_Mesh`) null)
        (set `self.Preview_Mesh` null)
        (set `self.Target_Rot` (struct))
        (set `/Game/Blueprints/BP_Character/BP_Character.Can_Shoot` true _as_bp_character_2)
        (set `/Game/Blueprints/BP_Character/BP_Character.Can_PickUp_Item` true _as_bp_character_2)))))

(event `EnhancedInput|/Game/Blueprints/inputs/Input_Actions/Build_System/IA_Build_Place`
  (params (ActionValue :type "Float (double-precision)") (ElapsedSeconds :type "Float (double-precision)") (TriggeredSeconds :type "Float (double-precision)") (InputAction :type "InputAction Object Reference" :default "/Game/Blueprints/inputs/Input_Actions/Build_System/IA_Build_Place.IA_Build_Place"))
  (:`Completed`
    (`self.b_Build_Mode`
      (:`then`
        (`|SpawnActorFromClass` "/Game/Blueprints/BP_Props/BPP_TallWall.BPP_TallWall_C" (`self.Build_Preview_Transform`) "Undefined" "MultiplyWithRoot" null null))
      (:`else`))))