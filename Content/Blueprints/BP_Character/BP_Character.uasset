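; Player character for a cursor-aimed game, with WASD movement, two weapon slots, a pause menu toggle and a shrink-then-destroy death.
; Tick traces under the cursor and, while the game instance allows movement, turns the body toward that point.
; The main weapon attachment also aims there, interpolating at the weapon's Heavyness.
; Weapons are picked up by line trace, swapped between main and back attachments, fired, or dropped onto the traced ground.
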(event `self.ReceiveBeginPlay`
  (bind _returnvalue (`GameplayStatics.GetPlayerController` 0))
  ; BEGIN PLAY
  (set `self.Player Speed` 1.0)
  (set `PlayerController.bShowMouseCursor` true _returnvalue)
  (`EnhancedInputSubsystemInterface.AddMappingContext` (pcsubsystem `EnhancedInputLocalPlayerSubsystem` _returnvalue) "/Game/Blueprints/inputs/IMC_Character_WASD.IMC_Character_WASD" 0 (make `ModifyContextOptions` true)))

(event `BeanDisapear`
  ; Make MrBean Disapear
  (bind (_direction _newtrack_0) (`Timeline|death` :!via `PlayFromStart`)
    (:`Update`
      (`self.SetActorScale3D` (`KismetMathLibrary.MakeVector` _newtrack_0 _newtrack_0 _newtrack_0)))
    (:`Finished`
      (`self.K2_DestroyActor`))))

(event `EnhancedInput|/Game/Blueprints/inputs/Input_Actions/IA_PauseGame`
  (params (ActionValue :type "Float (double-precision)") (ElapsedSeconds :type "Float (double-precision)") (TriggeredSeconds :type "Float (double-precision)") (InputAction :type "InputAction Object Reference" :default "/Game/Blueprints/inputs/Input_Actions/IA_PauseGame.IA_PauseGame"))
  ; IN GAME PAUSE MENU
  (:`Completed`
    (`/Engine/EditorBlueprintResources/StandardMacros.FlipFlop`
      (:`A`
        (bind _asbp_game_instance (cast `/Game/Blueprints/BP_GameInstance` (`GameplayStatics.GetGameInstance`)))
        (if (`/Game/Blueprints/BP_GameInstance.bCanPlayerMove?` _asbp_game_instance)
          (`WidgetLayoutLibrary.RemoveAllWidgets`)
          (bind _returnvalue (`|CreateWidget` "/Game/Blueprints/Widgets/WBP_SecondaryMenu.WBP_SecondaryMenu_C"))
          (`UserWidget.AddToViewport` _returnvalue 0)))
      (:`B`
        (`WidgetLayoutLibrary.RemoveAllWidgets`)
        (set `/Game/Blueprints/BP_GameInstance.bCanPlayerMove?` true _asbp_game_instance)))))

(event `self.ReceiveTick`
  (params (DeltaSeconds :type "Float (single-precision)"))
  ;[0.15 0.05313 0.05313 0.5] EVENT TICK
  (set `self.MouseImpactPoint` (`.ImpactPoint` (`GameplayStatics.BreakHitResult` (`PlayerController.GetHitResultUnderCursorByChannel` (`GameplayStatics.GetPlayerController` 0) "TraceTypeQuery2" true))))
  ;; condition de movement
  (bind _asbp_game_instance (cast `/Game/Blueprints/BP_GameInstance` (`GameplayStatics.GetGameInstance`)))
  (if (and (`self.IsLocallyControlled`) (`/Game/Blueprints/BP_GameInstance.bCanPlayerMove?` _asbp_game_instance))
    (`self.ActorRotation`)
    (`self.AimCursor`)))

(event `EnhancedInput|/Game/Blueprints/inputs/Input_Actions/IA_Move`
  (params (ActionValue :type "Vector2D Structure") (ElapsedSeconds :type "Float (double-precision)") (TriggeredSeconds :type "Float (double-precision)") (InputAction :type "InputAction Object Reference" :default "/Game/Blueprints/inputs/Input_Actions/IA_Move.IA_Move"))
  ; Movement
  (:`Triggered`
    (if (and (!= ActionValue (0.0 0.0)) (`self.IsLocallyControlled`))
      (`self.AddMovementInput` (`GameplayStatics.GetPlayerCharacter` 0) (* (`KismetMathLibrary.Normal` (`KismetMathLibrary.Conv_Vector2DToVector` ActionValue)) (`self.Player Speed`)) 1.0 false))))

(event `ActorRotation`
  (bind (_mouseimpactpoint_x _mouseimpactpoint_y _mouseimpactpoint_z) (`KismetMathLibrary.BreakVector` (`self.MouseImpactPoint`)))
  ; Player Look At Cursor
  (bind _output_get (set `self.Current Rotation` (`KismetMathLibrary.RInterpTo` (`self.Current Rotation`) (`KismetMathLibrary.FindLookAtRotation` (`self.K2_GetActorLocation`) (`KismetMathLibrary.MakeVector` _mouseimpactpoint_x _mouseimpactpoint_y (+ _mouseimpactpoint_z (`self.LOOK/AIM Height`)))) (`GameplayStatics.GetWorldDeltaSeconds`) (`self.ROT Interp Speed`))))
  (`self.K2_SetActorRotation` (`KismetMathLibrary.MakeRotator` 0.0 0.0 (.yaw _output_get))))

(event `EnhancedInput|/Game/Blueprints/inputs/Input_Actions/IA_SelectWaepon`
  (params (ActionValue :type "Float (double-precision)") (ElapsedSeconds :type "Float (double-precision)") (TriggeredSeconds :type "Float (double-precision)") (InputAction :type "InputAction Object Reference" :default "/Game/Blueprints/inputs/Input_Actions/IA_SelectWaepon.IA_SelectWaepon"))
  ;[0.15 0.15 0.15 0.5 50] IA_SwapWeapons
  (:`Triggered`
    (bind _weapon_main (`self.Weapon_Main`)
      (:`then`
        (`self.K2_AttachToComponent` _weapon_main (`self.Attachment_Back`) "None" "SnapToTarget" "SnapToTarget" "SnapToTarget" true)
        (bind _weapon_back (`self.Weapon_Back`)
          (:`then`
            (set `self.Set Weapon_Temp` _weapon_back)
            (set `self.Weapon_Back` (`self.Weapon_Main`))
            (set `self.Weapon_Main` null)
            (`self.K2_AttachToComponent` (`self.Set Weapon_Temp`) (`self.Attachment_Main`) "None" "SnapToTarget" "SnapToTarget" "SnapToTarget" true)
            (set `self.Weapon_Main` (`self.Set Weapon_Temp`))
            (set `self.Set Weapon_Temp` null))
          (:`else`
            (bind _weapon_main_2 (`self.Weapon_Main`)
              (:`then`
                (`self.K2_AttachToComponent` _weapon_main_2 (`self.Attachment_Back`) "None" "SnapToTarget" "SnapToTarget" "SnapToTarget" true)
                (set `self.Weapon_Back` (`self.Weapon_Main`))
                (set `self.Weapon_Main` null))
              (:`else`)))))
      (:`else`
        (bind _weapon_back_2 (`self.Weapon_Back`)
          (:`then`
            (`self.K2_AttachToComponent` _weapon_back_2 (`self.Attachment_Main`) "None" "SnapToTarget" "SnapToTarget" "SnapToTarget" true)
            (set `self.Weapon_Main` (`self.Weapon_Back`))
            (set `self.Weapon_Back` null))
          (:`else`))))))

(event `EnhancedInput|/Game/Blueprints/inputs/Input_Actions/IA_Shoot`
  (params (ActionValue :type "Float (double-precision)") (ElapsedSeconds :type "Float (double-precision)") (TriggeredSeconds :type "Float (double-precision)") (InputAction :type "InputAction Object Reference" :default "/Game/Blueprints/inputs/Input_Actions/IA_Shoot.IA_Shoot"))
  ; IA_SHOOT
  (:`Triggered`
    (`self.Can_Shoot`
      (:`then`
        (bind _weapon_main (`self.Weapon_Main`)
          (:`then`
            (`/Game/Blueprints/BP_Weapons/BP_Weapon_Parent.shoot` _weapon_main))
          (:`else`)))
      (:`else`))))

(event `EnhancedInput|/Game/Blueprints/inputs/Input_Actions/IA_Interact`
  (params (ActionValue :type "Float (double-precision)") (ElapsedSeconds :type "Float (double-precision)") (TriggeredSeconds :type "Float (double-precision)") (InputAction :type "InputAction Object Reference" :default "/Game/Blueprints/inputs/Input_Actions/IA_Interact.IA_Interact"))
  ; PICK UP WEAPON
  (:`Completed`
    (`self.Can_PickUp_Item`
      (:`then`
        (bind _outhit (`KismetSystemLibrary.LineTraceSingle` :`Start` (`SceneComponent.K2_GetComponentLocation` (`self.Camera`)) :`End` (`self.MouseImpactPoint`) :`TraceChannel` "TraceTypeQuery2" :`DrawDebugType` "ForDuration"))
        (bind _asbp_weapon_parent (cast `/Game/Blueprints/BP_Weapons/BP_Weapon_Parent` (`.HitActor` (`GameplayStatics.BreakHitResult` _outhit))))
        ;; Current Weapon == none ?
        (if (== (`self.Weapon_Main`) null)
          (`self.SetActorEnableCollision` _asbp_weapon_parent false)
          (`self.K2_AttachToComponent` _asbp_weapon_parent (`self.Attachment_Main`) "None" "SnapToTarget" "SnapToTarget" "SnapToTarget" true)
          (set `self.Weapon_Main` _asbp_weapon_parent)))
      (:`else`))))

(event `EnhancedInput|/Game/Blueprints/inputs/Input_Actions/IA_Drop`
  (params (ActionValue :type "Float (double-precision)") (ElapsedSeconds :type "Float (double-precision)") (TriggeredSeconds :type "Float (double-precision)") (InputAction :type "InputAction Object Reference" :default "/Game/Blueprints/inputs/Input_Actions/IA_Drop.IA_Drop"))
  (bind _weapon_main (`self.Weapon_Main`))
  (bind _returnvalue (`SceneComponent.K2_GetComponentLocation` (`self.Attachment_Main`)))
  ; Detach Weapon
  (:`Triggered`
    ;; Current Weapon == none ?
    (if (!= (`self.Weapon_Main`) null)
      (`self.K2_DetachFromActor` _weapon_main "KeepWorld" "KeepWorld" "KeepWorld")
      (`self.SetActorEnableCollision` _weapon_main true)
      (bind _outactors (`GameplayStatics.GetAllActorsOfClass` "/Game/Blueprints/BP_Weapons/BP_Weapon_Parent.BP_Weapon_Parent_C"))
      (bind _outhit (`KismetSystemLibrary.LineTraceSingle` _returnvalue (`KismetMathLibrary.MakeVector` (.x _returnvalue) (.y _returnvalue) -1000.0) "TraceTypeQuery1" false _outactors "ForDuration"))
      (`self.K2_SetActorLocationAndRotation` (`self.Weapon_Main`) (`.ImpactPoint` (`GameplayStatics.BreakHitResult` _outhit)) (struct :`Roll` -90.0) true true)
      (set `self.Weapon_Main` null))))

(event `AimCursor`
  (bind (_mouseimpactpoint_x _mouseimpactpoint_y _mouseimpactpoint_z) (`KismetMathLibrary.BreakVector` (`self.MouseImpactPoint`)))
  (bind _weapon_main (`self.Weapon_Main`))
  ; Main arraow attachement look at cursor
  (`/Engine/EditorBlueprintResources/StandardMacros.IsValid` _weapon_main
    (:`Is Valid`
      (bind _output_get (set `self.Attachement_Main_CurrentROT` (`KismetMathLibrary.RInterpTo` (`SceneComponent.K2_GetComponentRotation` (`self.Attachment_Main`)) (`KismetMathLibrary.FindLookAtRotation` (`SceneComponent.K2_GetComponentLocation` (`self.Attachment_Main`)) (`KismetMathLibrary.MakeVector` _mouseimpactpoint_x _mouseimpactpoint_y (+ _mouseimpactpoint_z (`self.LOOK/AIM Height`)))) (`GameplayStatics.GetWorldDeltaSeconds`) (`/Game/Blueprints/BP_Weapons/BP_Weapon_Parent.heavyness` _weapon_main))))
      (`SceneComponent.K2_SetWorldRotation` (`self.Attachment_Main`) _output_get false false))))

(fn `UserConstructionScript`)