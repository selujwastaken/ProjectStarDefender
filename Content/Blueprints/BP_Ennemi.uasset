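; BP_Ennemi is an enemy pawn that roams between turrets and dies when its health runs out.
; It picks random BP_Turret actors as AIMoveTo targets, calling GETARANDOMPOINT again on success or failure to keep moving.
; BeginPlay binds its HealthBar widget to itself via Initialise and starts the movement loop.
; Tick broadcasts current and max health through EDHealthUpdate every frame and destroys the actor at zero health.
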(event `self.ReceiveTick`
  (params (DeltaSeconds :type "Float (single-precision)"))
  (`self.ED_HealthUpdate` (`self.CurentHealth`) (`self.MaxHealth`))
  (if (<= (`self.CurentHealth`) 0.0)
    (`self.K2_DestroyActor`)))

(event `GET A RANDOM POINT`
  (bind _outactors (`GameplayStatics.GetAllActorsOfClass` "/Game/Blueprints/BP_Turret.BP_Turret_C" :!label _label))
  (bind _outitem (`KismetArrayLibrary.Array_Random` _outactors))
  (`|AIMoveTo` self (`self.K2_GetActorLocation` _outitem) _outitem
    (:`OnSuccess`
      _)
    (:`OnFail`
      _))
  (`self.GET A RANDOM POINT`))

(event `self.ReceiveBeginPlay`
  (bind _ashealth_bar (cast `/Game/Blueprints/Widgets/Widget_Ennemi/HealthBar` (`WidgetComponent.GetWidget` (`self.HealthBar`))))
  (`/Game/Blueprints/Widgets/Widget_Ennemi/HealthBar.Initialise` _ashealth_bar self)
  (goto _label))

(fn `UserConstructionScript`)